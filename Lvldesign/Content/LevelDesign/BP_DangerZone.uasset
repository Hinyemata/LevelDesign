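; BP_DangerZone is a level-design trigger volume that removes the first-person player when they enter it.
; On BeginPlay it caches the first BP_FirstPersonCharacter and GameManager found in the level.
; When that character begins overlapping the Box, it sets PlayerInTrigger, calls PlayerEnterDangerZone on the GameManager, then destroys the character actor.
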(event `self.ReceiveBeginPlay`
  ;[1 1 1] Set Player Reference
  (bind _outactors (`GameplayStatics.GetAllActorsOfClass` "/Game/FirstPerson/Blueprints/BP_FirstPersonCharacter.BP_FirstPersonCharacter_C"))
  (set `self.FirstPersonRef` (`|GetArrayItem` _outactors))
  (bind _outactors_2 (`GameplayStatics.GetAllActorsOfClass` "/Game/LevelDesign/GameManager.GameManager_C"))
  (set `self.GameManager_Ref` (`|GetArrayItem` _outactors_2)))

(event `self.Box.OnComponentBeginOverlap`
  (params (OverlappedComponent :type "PrimitiveComponent Object Reference") (OtherActor :type "Actor Object Reference") (OtherComp :type "PrimitiveComponent Object Reference") (OtherBodyIndex :type Integer) (bFromSweep :type Boolean) (SweepResult :type "HitResult Structure (by ref)"))
  ;[1 1 1] Do sth. if  player enters Zone
  (if (== OtherActor (`self.FirstPersonRef`))
    (set `self.PlayerInTrigger` true)
    ;[0.06935 1 0] Add desired Event here
    (`/Game/LevelDesign/GameManager.PlayerEnterDangerZone` (`self.GameManager_Ref`))
    (`self.K2_DestroyActor` (`self.FirstPersonRef`))))

(fn `UserConstructionScript`)