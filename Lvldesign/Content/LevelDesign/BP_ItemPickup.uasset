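; BP_ItemPickup is a spinning pickup actor that the first-person player collects, notifying the GameManager before destroying itself.
; A sphere overlap tracks whether the player is near, triggering pickup immediately or, when UseButtonToPickUp is set, showing a text prompt and waiting for the Buttonpress input.
; BeginPlay caches the character and GameManager by class lookup, and PickUpItem serves as the hook for custom pickup behavior.
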(event `self.ReceiveBeginPlay`
  ;[1 1 1] Set Player Reference and enable Input
  (bind _outactors (`GameplayStatics.GetAllActorsOfClass` "/Game/FirstPerson/Blueprints/BP_FirstPersonCharacter.BP_FirstPersonCharacter_C"))
  (set `self.FirstPersonRef` (`|GetArrayItem` _outactors))
  (bind _outactors_2 (`GameplayStatics.GetAllActorsOfClass` "/Game/LevelDesign/GameManager.GameManager_C"))
  (set `self.GameManager_Ref` (`|GetArrayItem` _outactors_2))
  (`self.EnableInput` (`GameplayStatics.GetPlayerController` 0)))

(event `self.ReceiveTick`
  (params (DeltaSeconds :type "Float (single-precision)"))
  ;[1 1 1] Rotate
  (`SceneComponent.K2_AddWorldRotation` (`self.StaticMesh`) (struct :`Yaw` 1.0) false false))

(event `self.Sphere.OnComponentBeginOverlap`
  (params (OverlappedComponent :type "PrimitiveComponent Object Reference") (OtherActor :type "Actor Object Reference") (OtherComp :type "PrimitiveComponent Object Reference") (OtherBodyIndex :type Integer) (bFromSweep :type Boolean) (SweepResult :type "HitResult Structure (by ref)"))
  ;[1 1 1] Enable Button Input if Player is near
  (if (== OtherActor (`self.FirstPersonRef`))
    (set `self.PlayerIsNear` true)
    (if (`self.UseButtonToPickUp`)
      (`SceneComponent.SetVisibility` (`self.TextRender`) true false)
      (`self.EnableInput` (`GameplayStatics.GetPlayerController` 0) null)
      (else
        (`self.PickUpItem`)))))

(event `self.Sphere.OnComponentEndOverlap`
  (params (OverlappedComponent :type "PrimitiveComponent Object Reference") (OtherActor :type "Actor Object Reference") (OtherComp :type "PrimitiveComponent Object Reference") (OtherBodyIndex :type Integer))
  ;[1 1 1] Disable  Button Input if Player is far away
  (if (== OtherActor (`self.FirstPersonRef`))
    (set `self.PlayerIsNear` false)
    (if (`self.UseButtonToPickUp`)
      (`SceneComponent.SetVisibility` (`self.TextRender`) false false)
      (`self.DisableInput` (`GameplayStatics.GetPlayerController` 0) null))))

(event `PickUpItem`
  ;[0.06935 1 0] Add desired Event here
  (`/Game/LevelDesign/GameManager.ItemPickedUp` (`self.GameManager_Ref`))
  (`self.K2_DestroyActor`))

(event `InputAction|Buttonpress`
  (params (Key :type "Key Structure"))
  ;[1 1 1] Do sth. if Button was pressed
  (:`Pressed`
    (if (`self.PlayerIsNear`)
      (if (`self.UseButtonToPickUp`)
        (`self.PickUpItem`)))))

(fn `UserConstructionScript`)