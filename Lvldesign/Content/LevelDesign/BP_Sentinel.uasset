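; BP_Sentinel is a level actor that can turn to face the first-person player character.
; StartFacingPlayer runs a self-repeating delayed loop that smoothly interpolates yaw toward the player, while StopFacingPlayer ends it and snaps back to the rotation saved at BeginPlay.
; Tick casts a debug-drawn visibility trace to the player, but its result is unused, as is the cached GameManager reference.
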(event `self.ReceiveBeginPlay`
  ;[1 1 1] Set Player Reference
  (bind _outactors (`GameplayStatics.GetAllActorsOfClass` "/Game/FirstPerson/Blueprints/BP_FirstPersonCharacter.BP_FirstPersonCharacter_C"))
  (set `self.FirstPersonRef` (`|GetArrayItem` _outactors))
  (bind _outactors_2 (`GameplayStatics.GetAllActorsOfClass` "/Game/LevelDesign/GameManager.GameManager_C"))
  (set `self.GameManager_Ref` (`|GetArrayItem` _outactors_2))
  (set `self.InitialRotation` (`self.K2_GetActorRotation`)))

(event `self.ReceiveTick`
  (params (DeltaSeconds :type "Float (single-precision)"))
  (`self.FireRaycast`))

(event `StartFacingPlayer`
  ;[1 1 1] Start facing Player
  (set `self.ShouldFacePlayer` true)
  (`self.FacePlayer`))

(event `StopFacingPlayer`
  ;[1 1 1] Stop facing Player
  (set `self.ShouldFacePlayer` false)
  (`self.K2_SetActorRotation` (`self.InitialRotation`)))

(event `FacePlayer`
  (bind (_returnvalue_roll _returnvalue_pitch _returnvalue_yaw) (`KismetMathLibrary.BreakRotator` (`KismetMathLibrary.RInterpTo` (`self.K2_GetActorRotation`) (`KismetMathLibrary.FindLookAtRotation` (`self.K2_GetActorLocation`) (`self.K2_GetActorLocation` (`self.FirstPersonRef`))) (`GameplayStatics.GetWorldDeltaSeconds`) (`self.TurnRotationDelay`))))
  ;[1 1 1] Adjust Rotation to Follow Player
  (if (`self.ShouldFacePlayer`)
    (`self.K2_SetActorRotation` (`KismetMathLibrary.MakeRotator` 0.0 0.0 _returnvalue_yaw))
    (`KismetSystemLibrary.Delay` 0.01)
    (`self.FacePlayer`)))

(event `FireRaycast`
  ;[1 1 1] Fire Raycast on Player
  (`KismetSystemLibrary.LineTraceSingle` :`Start` (`self.K2_GetActorLocation`) :`End` (`self.K2_GetActorLocation` (`self.FirstPersonRef`)) :`TraceChannel` "TraceTypeQuery1" :`DrawDebugType` "ForOneFrame"))

(fn `UserConstructionScript`)