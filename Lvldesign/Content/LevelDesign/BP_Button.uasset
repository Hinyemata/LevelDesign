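; BP_Button is a level button that switches the runtime state of a quest Data Layer on key press.
; BeginPlay caches the first-person character and GameManager, then enables input, while sphere overlaps track player proximity and toggle input.
; The press prints "Wegpunkt" and sets the layer to Loaded; a separate custom event sets it Activated.
; The proximity-checked GameManager notification is disconnected and never runs.
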(event `self.ReceiveBeginPlay`
  ;[1 1 1] Set Player Reference and enable Input
  (bind _outactors (`GameplayStatics.GetAllActorsOfClass` "/Game/FirstPerson/Blueprints/BP_FirstPersonCharacter.BP_FirstPersonCharacter_C"))
  (set `self.FirstPersonRef` (`|GetArrayItem` _outactors))
  (bind _outactors_2 (`GameplayStatics.GetAllActorsOfClass` "/Game/LevelDesign/GameManager.GameManager_C"))
  (set `self.GameManager_Ref` (`|GetArrayItem` _outactors_2))
  (`self.EnableInput` (`GameplayStatics.GetPlayerController` 0)))

(event `self.Sphere.OnComponentBeginOverlap`
  (params (OverlappedComponent :type "PrimitiveComponent Object Reference") (OtherActor :type "Actor Object Reference") (OtherComp :type "PrimitiveComponent Object Reference") (OtherBodyIndex :type Integer) (bFromSweep :type Boolean) (SweepResult :type "HitResult Structure (by ref)"))
  ;[1 1 1] Enable Button Input if Player is near
  (if (== OtherActor (`self.FirstPersonRef`))
    (set `self.PlayerIsNear` true)
    (`self.EnableInput` (`GameplayStatics.GetPlayerController` 0) null)))

(event `self.Sphere.OnComponentEndOverlap`
  (params (OverlappedComponent :type "PrimitiveComponent Object Reference") (OtherActor :type "Actor Object Reference") (OtherComp :type "PrimitiveComponent Object Reference") (OtherBodyIndex :type Integer))
  ;[1 1 1] Disable  Button Input if Player is far away
  (if (== OtherActor (`self.FirstPersonRef`))
    (set `self.PlayerIsNear` false)
    (`self.DisableInput` (`GameplayStatics.GetPlayerController` 0) null)))

(event `CustomEvent_0`
  (`DataLayerSubsystem.SetDataLayerRuntimeState` (subsystem `DataLayerSubsystem`) (`self.QuestDataLayer`) "Activated" false))

(event `InputAction|Buttonpress`
  (params (Key :type "Key Structure"))
  ;[1 1 1] Do sth. if Button was pressed
)

(event `InputAction|Buttonpress`
  (params (Key :type "Key Structure"))
  (:`Pressed`
    (`KismetSystemLibrary.PrintString` "Wegpunkt")
    (`DataLayerSubsystem.SetDataLayerRuntimeState` (subsystem `DataLayerSubsystem`) (`self.QuestDataLayer`) "Loaded" false)))

(fn `UserConstructionScript`)